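; BP_MainAnimal is an animal character Blueprint whose only logic in this file is on-screen debug output.
; Every Tick it prints the CharacterMovement max walk speed, the current speed from velocity length, and labels naming BP_MainAnimal as the active pawn.
; The active pawn label is fixed text with no possession check, and the construction script is empty.
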(event EventTick
  (params (DeltaSeconds :type Float%20%28single-precision%29))
  (Development|PrintString (Utilities|String|Append "Current Max Walk Speed : " (Utilities|String|ToString(Float) (Variables|/Script/Engine.CharacterMovementComponent|GetMaxWalkSpeed (Variables|Character|GetCharacterMovement)))) true true "(R=0.000000,G=0.660000,B=1.000000,A=1.000000)" 0.0)
  (Development|PrintString (Utilities|String|Append "Current Speed : " (Utilities|String|ToString(Float) (Math|Vector|VectorLength (Transformation|GetVelocity)))) true true "(R=0.000000,G=0.660000,B=1.000000,A=1.000000)" 0.0)
  (Development|PrintString "Current Active Pawn : BP_MainAnimal" true true "(R=0.000000,G=0.660000,B=1.000000,A=1.000000)" 0.0)
  (Development|PrintString "// BP_MainAnimal //" true true "(R=1.000000,G=0.000000,B=0.000000,A=1.000000)" 0.0))

(fn ConstructionScript)